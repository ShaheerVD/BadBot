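; Small scoring sphere that wanders through the level and increments the BP_BadBotGameMode score when a Pawn overlaps it.
; Timelines scale the mesh in on spawn and out before destruction, triggered by overlap or a Lifetime timer.
; Tick moves it along its forward vector while applying a random constant spin, so its path curves.
; IsWinking guards the wink-out only, so overlaps during the shrink still score.
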(event `self.ReceiveBeginPlay`
  (`self.WinkIn`)
  ;[0.4688 0.02441 0.02441 0.5] Start wink out timeline
  (`self.InitializeDeltaRotation`)
  (`KismetSystemLibrary.K2_SetTimerDelegate` (delegate `WinkOut`) (`self.Lifetime`))
  (add `PrimitiveComponent.OnComponentBeginOverlap` (`self.SphereVolume`) (delegate `OnSphereOverlap`)))

(event `OnSphereOverlap`
  (params (OverlappedComponent :type "PrimitiveComponent Object Reference") (OtherActor :type "Actor Object Reference") (OtherComp :type "PrimitiveComponent Object Reference") (OtherBodyIndex :type Integer) (bFromSweep :type Boolean) (SweepResult :type "HitResult Structure (by ref)"))
  (if (`GameplayStatics.ObjectIsA` OtherActor "/Script/Engine.Pawn")
    (bind _asbp_bad_bot_game_mode (cast `/Game/Blueprints/Game/BP_BadBotGameMode` (`GameplayStatics.GetGameMode`)))
    (`/Game/Blueprints/Game/BP_BadBotGameMode.IncrementScore` _asbp_bad_bot_game_mode)
    (`self.WinkOut`)))

(event `WinkOut`
  ;[0.4688 0.02441 0.02441 0.5] Start wink out timeline
  (if (not (`self.isWinking`))
    (set `self.isWinking` true)
    (bind (_direction _scale) (`Timeline|WinkOutTimeline`)
      (:`Update`
        (`self.ScaleSphere` _scale))
      (:`Finished`
        (`self.K2_DestroyActor`)))))

(event `self.ReceiveTick`
  (params (DeltaSeconds :type "Float (single-precision)"))
  ;[0.092 0.839 0.901 0.5] Update location and Rotation
  (`self.UpdateLocation` DeltaSeconds)
  (`self.UpdateRotation` DeltaSeconds))

(event `WinkIn`
  ;[0.4688 0.02441 0.02441 0.5] Wink into Existence
  (bind (_direction _scale) (`Timeline|WinkInTimeline`)
    (:`Update`
      (`SceneComponent.SetWorldScale3D` (`self.SphereMesh`) _scale))))

(fn `InitializeDeltaRotation`
  (set `self.Delta Rotation` (* (`KismetMathLibrary.RandomRotator` false) (`self.RotationScaleFactor`))))

(fn `ScaleSphere`
  (params (Scale :type "Float (single-precision)"))
  (`SceneComponent.SetWorldScale3D` (`self.SphereMesh`) (`KismetMathLibrary.MakeVector` Scale Scale Scale)))

(fn `UpdateLocation`
  (params (DeltaSeconds :type "Float (double-precision)"))
  (`self.K2_AddActorWorldOffset` (* (`self.GetActorForwardVector`) (* DeltaSeconds (`self.Speed`)))))

(fn `UpdateRotation`
  (params (DeltaSeconds :type "Float (single-precision)"))
  (`self.K2_AddActorWorldRotation` (* (`self.Delta Rotation`) DeltaSeconds)))

(fn `UserConstructionScript`)